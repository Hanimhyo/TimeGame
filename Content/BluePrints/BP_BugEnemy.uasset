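; Bug enemy that chases the player on a physics sphere, easing to a stop within attack range.
; Each Tick it updates the target vector, turns, sets clamped horizontal velocity and jumps when the player is well above.
; A fast BP_UseInverseActor hit knocks it back and pauses chasing for two seconds; other non-wall hits re-arm jumping after a delay.
; Hitting a "Wall"-tagged actor increments the game mode's score and destroys it.
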(event EventBeginPlay)

(event Collision|EventActorBeginOverlap
  (params (OtherActor :type Actor%20Object%20Reference)))

(event EventTick
  (params (DeltaSeconds :type Float%20%28single-precision%29))
  (if (Variables|Default|GetisDamage)
    (Utilities|FlowControl|Delay 2.0)
    (Variables|Default|SetisDamage false)
    (else
      (CallFunction|MakeGoVector)
      (CallFunction|Rotate)
      (CallFunction|Move)
      (CallFunction|Yveclity DeltaSeconds)
      (CallFunction|Jump))))

(event Collision|EventHit
  (params (MyComp :type Primitive%20Component%20Object%20Reference) (Other :type Actor%20Object%20Reference) (OtherComp :type Primitive%20Component%20Object%20Reference) (bSelfMoved :type Boolean) (HitLocation :type Vector :default "0, 0, 0") (HitNormal :type Vector :default "0, 0, 0") (NormalImpulse :type Vector :default "0, 0, 0") (Hit :type Hit%20Result%20Structure%20%28by%20ref%29))
  (if (Actor|ActorHasTag Other "Wall")
    (bind _asbp_time_game_game_mode (Utilities|Casting|CastToBP_TimeGameGameMode (Game|GetGameMode)))
    (Variables|/Game/BluePrints/BP_TimeGameGameMode.BP_TimeGameGameMode_C|Setscore _asbp_time_game_game_mode (+ (Variables|/Game/BluePrints/BP_TimeGameGameMode.BP_TimeGameGameMode_C|Getscore _asbp_time_game_game_mode) 1))
    (Actor|DestroyActor)
    (else
      (bind _asbp_use_inverse_actor (Utilities|Casting|CastToBP_UseInverseActor Other)
        (:then
          (if (> (Math|Vector|VectorLength (Transformation|GetVelocity _asbp_use_inverse_actor)) 5e+02)
            (Variables|Default|SetisDamage true)
            (Physics|SetPhysicsLinearVelocity (Variables|Default|GetSphere) (+ (Transformation|GetVelocity) (Transformation|GetVelocity _asbp_use_inverse_actor)) false "None")
            (else
              (Utilities|FlowControl|Delay 0.2 :!label _label)
              (Variables|Default|SetisJump false))))
        (:CastFailed
          (goto _label))))))

(fn ConstructionScript)

(fn MakeGoVector
  (bind _returnvalue (Game|Player|GetPlayerPawn 0))
  (bind _returnvalue_2 (Transformation|GetActorLocation))
  (bind _returnvalue_3 (Transformation|GetActorLocation _returnvalue))
  (bind _returnvalue_4 (- _returnvalue_3 _returnvalue_2))
  (if (> (.z _returnvalue_4) 2e+02)
    (Variables|Default|SetisTargetUp true)
    (else
      (Variables|Default|SetisTargetUp false)))
  (Variables|Default|SetgoVector (Math|Vector|Normalize (Math|Vector|MakeVector (.x _returnvalue_4) (.y _returnvalue_4) 0.0)))
  (bind _output_get (Variables|Default|SettargetDistance (Math|Vector|Distance(Vector) _returnvalue_3 _returnvalue_2)))
  (if (< _output_get (Variables|Default|GetattackRange))
    (Variables|Default|SetcurrentSpeed (Math|Float|Lerp (Variables|Default|GetcurrentSpeed) 0.0 0.1))
    (else
      (Variables|Default|SetcurrentSpeed (Math|Float|Lerp (Variables|Default|GetcurrentSpeed) (Variables|Default|Getspeed) 0.1)))))

(fn Move
  (bind _sphere (Variables|Default|GetSphere))
  (bind _govector (Variables|Default|GetgoVector))
  (bind _currentspeed (Variables|Default|GetcurrentSpeed))
  (bind _currentspeed_2 (Variables|Default|GetcurrentSpeed))
  (bind _returnvalue (* _govector _currentspeed))
  (bind _returnvalue_2 (* _currentspeed_2 -1.0))
  (bind _returnvalue_3 (Physics|GetPhysicsLinearVelocity _sphere "None"))
  (Physics|SetPhysicsLinearVelocity _sphere (Math|Vector|MakeVector (Math|Float|Clamp(Float) (.x (+ _returnvalue_3 (Math|Vector|MakeVector (.x _returnvalue) (.y _returnvalue) 0.0))) _returnvalue_2 _currentspeed_2) (Math|Float|Clamp(Float) (.y (+ _returnvalue_3 (Math|Vector|MakeVector (.x _returnvalue) (.y _returnvalue) 0.0))) _returnvalue_2 _currentspeed_2) (.z (+ _returnvalue_3 (Math|Vector|MakeVector (.x _returnvalue) (.y _returnvalue) 0.0)))) false "None"))

(fn Rotate
  (bind _govector (Variables|Default|GetgoVector))
  (Transformation|SetActorRotation (Math|Rotator|MakeRotfromXZ (Math|Vector|MakeVector (.x _govector) (.y _govector) 0.0) (Math|Vector|MakeVector 0.0 0.0 1.0))))

(fn Yveclity
  (params (detaTime :type Float%20%28single-precision%29))
  (if (Variables|Default|GetisJump)
    (Variables|Default|SetyVelocity (+ (* detaTime (Variables|Default|GetgravityValue)) (Variables|Default|GetyVelocity)))))

(fn Jump
  (bind _sphere (Variables|Default|GetSphere))
  (if (Variables|Default|GetisTargetUp)
    (if (not (Variables|Default|GetisJump))
      (Variables|Default|SetisJump true)
      (bind _output_get (Variables|Default|SetyVelocity 7e+02))
      (bind _returnvalue (Physics|GetPhysicsLinearVelocity _sphere "None"))
      (Physics|SetPhysicsLinearVelocity _sphere (Math|Vector|MakeVector (.x _returnvalue) (.y _returnvalue) _output_get) false "None"))))