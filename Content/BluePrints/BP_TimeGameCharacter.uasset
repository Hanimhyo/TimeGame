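; Player character for a time-manipulation shooter, with weapons, time skills and object grabbing.
; Fire01 zooms when held and shoots on release: bazooka projectile or sniper push trace, with a mine case the weapon toggle never selects.
; Fire02 spawns inverse, time-stop or antigravity spheres, with rim color marking the skill; InverseButton inverts CubeList actors.
; Grabbing pulls the player toward a traced BP_UseInverseActor each Tick, attaches on hit and relaunches on release.
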(event Custom|ReleaseNext
  ;[1 1 1] GripObject
  (Utilities|FlowControl|Delay 0.0)
  (Variables|/Script/Engine.MovementComponent|SetVelocity (Variables|Character|GetCharacterMovement) (Variables|Default|GetreleaseVelocity)))

(event EventBeginPlay
  (bind _returnvalue (Rendering|Material|CreateDynamicMaterialInstance (Variables|Character|GetMesh) 0 0 "None" :!class /Script/Engine.PrimitiveComponent))
  (Variables|Default|SetplayMaterial _returnvalue))

(event Collision|EventActorBeginOverlap
  (params (OtherActor :type Actor%20Object%20Reference)))

(event EventTick
  (params (DeltaSeconds :type Float%20%28single-precision%29))
  (CallFunction|PlayerUp)
  (CallFunction|CameraZoom)
  (CallFunction|MoveGrab)
  (CallFunction|ZVelocitySetting))

(event Collision|EventHit
  (params (MyComp :type Primitive%20Component%20Object%20Reference) (Other :type Actor%20Object%20Reference) (OtherComp :type Primitive%20Component%20Object%20Reference) (bSelfMoved :type Boolean) (HitLocation :type Vector :default "0, 0, 0") (HitNormal :type Vector :default "0, 0, 0") (NormalImpulse :type Vector :default "0, 0, 0") (Hit :type Hit%20Result%20Structure%20%28by%20ref%29))
  ;[1 1 1] HitGrapObject
  (if (Variables|Default|GetisGrab)
    (if (not (== Other (Variables|Default|GetgrabActor)))
      (bind _returnvalue (Physics|GetPhysicsLinearVelocity OtherComp "None"))
      (if (not (> (Math|Vector|VectorLength (- _returnvalue (Transformation|GetVelocity))) 2e+03))
        (CallFunction|RelaeseObject)))
    (elif (not (Variables|Default|GetisHitGrabObject))
      (Variables|Default|SetisHitGrabObject (== Other (Variables|Default|GetgrabActor))))))

(event Input|ActionEvents|InputActionSkillChange
  (params (Key :type Key%20Structure))
  ;[1 1 1] ChangeSkill
  (:Pressed
    (switch Utilities|FlowControl|Switch|SwitchonEPlayerSkillState (Variables|Default|GetplayerSkillState)
      (:Inverse
        (bind _output_get (Variables|Default|SetmySkillstate "Stop"))
        (Variables|Default|SetplayerSkillState _output_get)
        (Rendering|Material|SetVectorParameterValue (Variables|Default|GetplayMaterial) "RimColor" "(R=10.000000,G=1.000000,B=0.000000,A=1.000000)" :!class /Script/Engine.MaterialInstanceDynamic))
      (:Stop
        (bind _output_get_2 (Variables|Default|SetmySkillstate "Antigravity"))
        (Variables|Default|SetplayerSkillState _output_get_2)
        (Rendering|Material|SetVectorParameterValue (Variables|Default|GetplayMaterial) "RimColor" "(R=0.000000,G=0.000000,B=10.000000,A=1.000000)" :!class /Script/Engine.MaterialInstanceDynamic))
      (:Antigravity
        (bind _output_get_3 (Variables|Default|SetmySkillstate "Inverse"))
        (Variables|Default|SetplayerSkillState _output_get_3)
        (Rendering|Material|SetVectorParameterValue (Variables|Default|GetplayMaterial) "RimColor" "(R=10.000000,G=0.000000,B=0.000000,A=1.000000)" :!class /Script/Engine.MaterialInstanceDynamic)))))

(event Input|ActionEvents|InputActionFire02
  (params (Key :type Key%20Structure))
  (bind _returnvalue (Transformation|GetActorLocation))
  ;[1 1 1] Use_Skill
  (:Pressed
    (switch Utilities|FlowControl|Switch|SwitchonEPlayerSkillState (Variables|Default|GetplayerSkillState)
      (:Inverse
        (Game|SpawnActorfromClass "/Game/BluePrints/BP_GrowSphere_Inverse.BP_GrowSphere_Inverse_C" (Math|Transform|MakeTransform _returnvalue "0, 0, 0" "40.000000,40.000000,40.000000") "Undefined" 0 0))
      (:Stop
        (Game|SpawnActorfromClass "/Game/BluePrints/BP_GrowSphere_TimeStop.BP_GrowSphere_TimeStop_C" (Math|Transform|MakeTransform _returnvalue "0, 0, 0" "20.000000,20.000000,20.000000") "Undefined" 0 0))
      (:Antigravity
        (Game|SpawnActorfromClass "/Game/BluePrints/BP_GrowSphere_NoGravity.BP_GrowSphere_NoGravity_C" (Math|Transform|MakeTransform _returnvalue "0, 0, 0" "20.000000,20.000000,20.000000") "Undefined" 0 0)))))

(event Input|ActionEvents|InputActionWeaponChange
  (params (Key :type Key%20Structure))
  ;[1 1 1] ChangeWeapon
  (:Pressed
    (switch Utilities|FlowControl|Switch|SwitchonEPlayerWeaponState (Variables|Default|GetplayerWeaponState)
      (:Bazooka
        (bind _output_get (Variables|Default|SetmyWeaponstate "Sniper"))
        (Variables|Default|SetplayerWeaponState _output_get))
      (:Sniper
        (bind _output_get_2 (Variables|Default|SetmyWeaponstate "Bazooka"))
        (Variables|Default|SetplayerWeaponState _output_get_2))
      (:Mine
        (bind _output_get_3 (Variables|Default|SetmyWeaponstate "Bazooka"))
        (Variables|Default|SetplayerWeaponState _output_get_3)))))

(event Input|ActionEvents|InputActionFire01
  (params (Key :type Key%20Structure))
  ;[1 1 1] Weapom_Fire
  (:Pressed
    (Variables|Default|SetisZoom true)
    (Variables|Default|SetzoomCurrentTime 0.0))
  (:Released
    (Variables|Default|SetisZoom false)
    (switch Utilities|FlowControl|Switch|SwitchonEPlayerWeaponState (Variables|Default|GetplayerWeaponState)
      (:Bazooka
        (CallFunction|FireBazooka))
      (:Sniper
        (CallFunction|FireSniper))
      (:Mine
        (CallFunction|FireMine)))))

(event Input|ActionEvents|InputActionInverseButton
  (params (Key :type Key%20Structure))
  ;[1 1 1] World_Inverse
  (:Pressed
    (for _index (range 0 (Utilities|Array|Length (Variables|Default|GetcubeList)))
      (bind _asbp_use_inverse_actor (Utilities|Casting|CastToBP_UseInverseActor (Utilities|Array|Get(acopy) (Variables|Default|GetcubeList) _index)))
      (Default|WorldInverse _asbp_use_inverse_actor))))

(event Input|ActionEvents|InputActionGrabObject
  (params (Key :type Key%20Structure))
  ;[1 1 1] GripObject
  (:Pressed
    (CallFunction|GrapObject))
  (:Released
    (CallFunction|RelaeseObject)))

(fn ConstructionScript)

(fn GrapObject
  (bind _followcamera (Variables|Default|GetFollowCamera))
  (bind _outhit (Collision|LineTraceByChannel (Transformation|GetWorldLocation _followcamera) (+ (Transformation|GetWorldLocation _followcamera) (* (Math|Vector|GetForwardVector _followcamera) 1e+06)) "TraceTypeQuery1" false 0 "None"))
  (bind _asbp_use_inverse_actor (Utilities|Casting|CastToBP_UseInverseActor (.HitActor (Collision|BreakHitResult _outhit))))
  (Variables|Default|SetgrabActor _asbp_use_inverse_actor)
  (Variables|Default|SetisGrabObject_Go true))

(fn RelaeseObject
  (if (Variables|Default|GetisGrab)
    (Variables|Default|SetreleaseVelocity (+ (Transformation|GetVelocity) (Math|Vector|MakeVector 0.0 0.0 3.5e+02)))
    (Transformation|DetachFromActor "KeepWorld" "KeepWorld" "KeepWorld")
    (Variables|/Script/Engine.MovementComponent|SetVelocity (Variables|Character|GetCharacterMovement) (Variables|Default|GetreleaseVelocity))
    (CallFunction|ReleaseNext)
    (Variables|Default|SetisGrabObject_Go false)
    (Variables|Default|SetisGrab false)
    (Variables|Default|SetgrabActor (Variables|Default|GetnullActor))
    (Variables|Default|SetisHitGrabObject false)
    (bind _asabp_player (Utilities|Casting|CastToABP_Player (Components|SkeletalMesh|GetAnimInstance (Variables|Character|GetMesh))))
    (Variables|/Game/BluePrints/Animetion/ABP_Player.ABP_Player_C|SetisGrab _asabp_player false)
    (else
      (Variables|Default|SetisGrabObject_Go false))))

(fn PlayerUp
  (bind _returnvalue (Transformation|GetActorForwardVector))
  (if (not (Variables|Default|GetisGrabObject_Go))
    (Transformation|SetActorRotation (Math|Rotator|Lerp(Rotator) (Math|Rotator|MakeRotfromXZ (Transformation|GetActorForwardVector) (Transformation|GetActorUpVector)) (Math|Rotator|MakeRotfromXZ (Math|Vector|Normalize (Math|Vector|MakeVector (.x _returnvalue) (.y _returnvalue) 0.0)) (Math|Vector|MakeVector 0.0 0.0 1.0)) 0.1))))

(fn CameraRotate
  (bind (_outhit _returnvalue) (Collision|LineTraceByChannel (Transformation|GetWorldLocation (Variables|Default|GetFollowCamera)) (+ (Transformation|GetWorldLocation (Variables|Default|GetFollowCamera)) (* (Math|Vector|GetForwardVector (Variables|Default|GetFollowCamera)) 1e+06)) "TraceTypeQuery1" false 0 "None"))
  (if _returnvalue
    (Transformation|SetWorldRotation (Variables|Default|GetFirePos) (Math|Rotator|FindLookatRotation (Transformation|GetActorLocation) (.ImpactPoint (Collision|BreakHitResult _outhit))) false false)
    (else
      (Transformation|SetWorldRotation (Variables|Default|GetFirePos) (Transformation|GetWorldRotation (Variables|Default|GetFollowCamera)) false false))))

(fn FireBazooka
  (CallFunction|CameraRotate)
  (Game|SpawnActorfromClass "/Game/BluePrints/BP_Bazooka.BP_Bazooka_C" (Transformation|GetWorldTransform (Variables|Default|GetFirePos)) "AlwaysSpawn" 0 0)
  (bind _asabp_player (Utilities|Casting|CastToABP_Player (Components|SkeletalMesh|GetAnimInstance (Variables|Character|GetMesh))))
  (Default|ShotName _asabp_player "BazookaShoot"))

(fn FireSniper
  (bind _followcamera (Variables|Default|GetFollowCamera))
  (bind _followcamera_2 (Variables|Default|GetFollowCamera))
  (bind _followcamera_3 (Variables|Default|GetFollowCamera))
  (bind _followcamera_4 (Variables|Default|GetFollowCamera))
  (bind _returnvalue (Transformation|GetWorldLocation _followcamera_3))
  (bind _returnvalue_2 (Math|Vector|GetForwardVector _followcamera))
  (bind _returnvalue_3 (Transformation|GetWorldLocation _followcamera_4))
  (bind _returnvalue_4 (Math|Vector|GetForwardVector _followcamera_2))
  (bind _returnvalue_5 (* _returnvalue_4 1e+06))
  (bind _returnvalue_6 (+ _returnvalue _returnvalue_5))
  (bind _outhits (Class|KismetSystemLibrary|LineTraceMultiforObjects _returnvalue_3 _returnvalue_6 (Utilities|Array|MakeArray "ObjectTypeQuery4" "ObjectTypeQuery3") false 0 "None" true))
  (for _array_element _outhits
    (bind _asbp_use_inverse_actor (Utilities|Casting|CastToBP_UseInverseActor (.HitActor (Collision|BreakHitResult _array_element)))
      (:then
        (bind _asstatic_mesh_component (Utilities|Casting|CastToStaticMeshComponent (Variables|/Script/Engine.Actor|GetRootComponent _asbp_use_inverse_actor)))
        (Physics|SetPhysicsLinearVelocity _asstatic_mesh_component (* _returnvalue_2 5e+03) false "None")
        (Default|GetStopPhysics _asbp_use_inverse_actor _returnvalue_2 5e+03))
      (:CastFailed
        (bind _ascharacter (Utilities|Casting|CastToCharacter (.HitActor (Collision|BreakHitResult _array_element)))
          (:then
            (Pawn|Components|CharacterMovement|SetMovementMode (Variables|/Script/Engine.Character|GetCharacterMovement _ascharacter) "MOVE_Falling" 0)
            (Variables|/Script/Engine.MovementComponent|SetVelocity (Variables|/Script/Engine.Character|GetCharacterMovement _ascharacter) (+ (* _returnvalue_2 1.5e+03) (Pawn|Components|CharacterMovement|GetLastUpdateVelocity (Variables|/Script/Engine.Character|GetCharacterMovement _ascharacter)))))
          (:CastFailed
            (bind _asbp_enemy_bug_bug_bug (Utilities|Casting|CastToBP_EnemyBugBugBug (.HitActor (Collision|BreakHitResult _array_element))))
            (Variables|/Game/BluePrints/BP_EnemyBugBugBug.BP_EnemyBugBugBug_C|SetisDamage _asbp_enemy_bug_bug_bug true)
            (Physics|SetPhysicsLinearVelocity (Variables|/Game/BluePrints/BP_EnemyBugBugBug.BP_EnemyBugBugBug_C|GetSphere _asbp_enemy_bug_bug_bug) (* (Math|Vector|GetForwardVector (Variables|Default|GetFollowCamera)) 5e+03) false "None"))))))
  (Audio|PlaySoundatLocation "/Game/Resouce/Rifle.Rifle" (Transformation|GetActorLocation) "0, 0, 0" 1.0 1.0 0.0 0 0 0)
  (bind _returnvalue_7 (AddComponent|AddNiagaraComponent false))
  (Class|NiagaraComponent|SetNiagaraVariableVec3 _returnvalue_7 "Beam Start" (+ (+ _returnvalue_3 "0.000000, 0,-5.000000") (* _returnvalue_4 1e+02)))
  (Class|NiagaraComponent|SetNiagaraVariableVec3 _returnvalue_7 "Beam End" _returnvalue_6)
  (bind _asabp_player (Utilities|Casting|CastToABP_Player (Components|SkeletalMesh|GetAnimInstance (Variables|Character|GetMesh))))
  (Default|ShotName _asabp_player "SniperShoot"))

(fn CameraZoom
  (Utilities|FlowControl|Sequence
    (:then_0
      (if (Variables|Default|GetisZoom)
        (bind _output_get (Variables|Default|SetzoomCurrentTime (+ (Utilities|Time|GetWorldDeltaSeconds) (Variables|Default|GetzoomCurrentTime))))
        (if (> _output_get (Variables|Default|GetzoomStartTime))
          (Variables|Default|SetgoalFOV 3e+01))
        (else
          (Variables|Default|SetgoalFOV 9e+01))))
    (:then_1
      (bind _output_get_2 (Variables|Default|SetcurrentFOV (Math|Float|Lerp (Variables|Default|GetcurrentFOV) (Variables|Default|GetgoalFOV) 0.2)))
      (Camera|SetFieldOfView (Variables|Default|GetFollowCamera) _output_get_2))))

(fn FireMine
  (bind (_outhit _returnvalue) (Collision|LineTraceByChannel (Transformation|GetWorldLocation (Variables|Default|GetFollowCamera)) (+ (Transformation|GetWorldLocation (Variables|Default|GetFollowCamera)) (* (Math|Vector|GetForwardVector (Variables|Default|GetFollowCamera)) 1e+06)) "TraceTypeQuery1" false 0 "None"))
  (if _returnvalue
    (bind _returnvalue_2 (Game|SpawnActorfromClass "/Game/BluePrints/BP_TimeMine.BP_TimeMine_C" (Math|Transform|MakeTransform (.ImpactPoint (Collision|BreakHitResult _outhit)) (Math|Conversions|RotationFromXVector (.ImpactNormal (Collision|BreakHitResult _outhit))) "0.400000,0.400000,0.400000") "Undefined" 0 0))
    (Transformation|AttachActorToActor _returnvalue_2 (.HitActor (Collision|BreakHitResult _outhit)) "None" "KeepWorld" "KeepWorld" "KeepWorld" true)))

(fn MoveGrab
  (bind _returnvalue (Transformation|GetActorLocation))
  (bind _grabactor (Variables|Default|GetgrabActor))
  (bind _returnvalue_2 (Transformation|GetActorLocation _grabactor))
  (bind _returnvalue_3 (- _returnvalue_2 _returnvalue))
  (if (Variables|Default|GetisGrabObject_Go)
    (Variables|/Script/Engine.MovementComponent|SetVelocity (Variables|Character|GetCharacterMovement) (+ (* (Math|Vector|Normalize (Math|Vector|MakeVector (.x _returnvalue_3) (.y _returnvalue_3) 0.0)) 6e+02) (Math|Vector|MakeVector 0.0 0.0 (* 100 (Variables|Default|GetzVelocity)))))
    (if (Variables|Default|GetisHitGrabObject)
      (Transformation|AttachActorToActor (Variables|Default|GetgrabActor) "None" "KeepWorld" "KeepWorld" "KeepWorld" true)
      (bind _output_get (Variables|Default|SetisGrab true))
      (bind _asabp_player (Utilities|Casting|CastToABP_Player (Components|SkeletalMesh|GetAnimInstance (Variables|Character|GetMesh))))
      (Variables|/Game/BluePrints/Animetion/ABP_Player.ABP_Player_C|SetisGrab _asabp_player _output_get)
      (Variables|Default|SetgrabRelativePos (.location (Transformation|GetRelativeTransform (Variables|Default|GetCapsuleComponent)))))))

(fn ZVelocitySetting
  (if (AI|Components|NavMovement|IsMovingonGround (Variables|Character|GetCharacterMovement))
    (Variables|Default|SetzVelocity 0.0)
    (else
      (Variables|Default|SetzVelocity (+ (Variables|Default|GetzVelocity) (* (Utilities|Time|GetWorldDeltaSeconds) -5.0))))))

(fn GrabIng
  (if (Variables|Default|GetisGrab)
    (Transformation|SetActorRelativeLocation (Variables|Default|GetgrabRelativePos))))

(fn AddScore
  (Variables|Default|Setscore (+ (Variables|Default|Getscore) 1)))