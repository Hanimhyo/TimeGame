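; BP_GrowSphere_Inverse is a sphere actor that triggers inverse behavior on nearby actors when it spawns.
; On BeginPlay it overlaps PhysicsBody objects within a scale-based radius and calls OnInverseStart on BP_UseInverseActor results, stopping at the first failed cast.
; Tick changes its uniform scale by GrowSpeed over time and destroys it once the scale drops below zero.
; An IsInverse-guarded OnInverseStart branch is left unconnected.
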(event EventTick
  (params (DeltaSeconds :type Float%20%28single-precision%29))
  (bind _returnvalue (Transformation|GetActorScale3D))
  (bind _growspeed (Variables|Default|GetgrowSpeed))
  (bind _returnvalue_2 (* DeltaSeconds _growspeed))
  (bind _returnvalue_3 (+ _returnvalue_2 (.x _returnvalue)))
  (Transformation|SetActorScale3D (Math|Vector|MakeVector _returnvalue_3 _returnvalue_3 _returnvalue_3))
  (if (< (.x (Transformation|GetActorScale3D)) 0.0)
    (Actor|DestroyActor)))

(event EventBeginPlay
  (bind _outactors (Collision|SphereOverlapActors (Transformation|GetActorLocation) (* (.x (Transformation|GetActorScale3D)) 5e+01) (Utilities|Array|MakeArray "ObjectTypeQuery4") 0))
  (for _array_element _outactors
    (bind _asbp_use_inverse_actor (Utilities|Casting|CastToBP_UseInverseActor _array_element))
    (Default|OnInverseStart _asbp_use_inverse_actor)))

(fn ConstructionScript)