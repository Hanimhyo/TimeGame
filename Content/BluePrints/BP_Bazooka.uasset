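; Bazooka projectile that explodes on hit, pushing nearby BP_UseInverseActor physics objects, then destroys itself with a particle burst.
; MakeExplosionLocation offsets the blast origin behind and below the projectile, angling the push, and plays the explosion sound.
; Each overlapped actor with a static mesh root gets a constant radial velocity impulse.
; It also receives direction and linear distance-falloff strength through GetStopPhysics.
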(event EventBeginPlay)

(event Collision|EventActorBeginOverlap
  (params (OtherActor :type Actor%20Object%20Reference)))

(event EventTick
  (params (DeltaSeconds :type Float%20%28single-precision%29)))

(event Collision|EventHit
  (params (MyComp :type Primitive%20Component%20Object%20Reference) (Other :type Actor%20Object%20Reference) (OtherComp :type Primitive%20Component%20Object%20Reference) (bSelfMoved :type Boolean) (HitLocation :type Vector :default "0, 0, 0") (HitNormal :type Vector :default "0, 0, 0") (NormalImpulse :type Vector :default "0, 0, 0") (Hit :type Hit%20Result%20Structure%20%28by%20ref%29))
  (CallFunction|MakeExplosionLocation)
  (bind _outactors (Collision|SphereOverlapActors (Transformation|GetActorLocation) 5e+02 (Utilities|Array|MakeArray "ObjectTypeQuery4") "/Game/BluePrints/BP_UseInverseActor.BP_UseInverseActor_C"))
  (for _array_element _outactors
    (bind _asstatic_mesh_component (Utilities|Casting|CastToStaticMeshComponent (Variables|/Script/Engine.Actor|GetRootComponent _array_element)))
    (Physics|AddRadialImpulse _asstatic_mesh_component (Variables|Default|GetexplosionPos) 7e+02 1.5e+03 "RIF_Constant" true)
    (bind _asbp_use_inverse_actor (Utilities|Casting|CastToBP_UseInverseActor _array_element))
    (Default|GetStopPhysics _asbp_use_inverse_actor (Math|Vector|Normalize (- (Transformation|GetActorLocation _asbp_use_inverse_actor) (Variables|Default|GetexplosionPos))) (* 1500 (/ (- 7e+02 (Math|Vector|VectorLength (- (Transformation|GetActorLocation _asbp_use_inverse_actor) (Variables|Default|GetexplosionPos)))) 7e+02))))
  (Effects|SpawnEmitteratLocation "/Game/StarterContent/Particles/P_Explosion.P_Explosion" (Transformation|GetActorLocation) "0, 0, 0" "5.000000,5.000000,5.000000")
  (Actor|DestroyActor))

(fn ConstructionScript)

(fn MakeExplosionLocation
  (Variables|Default|SetexplosionPos (+ (Transformation|GetActorLocation) (+ (* (Transformation|GetActorForwardVector) -1e+02) (* (Math|Vector|MakeVector 0.0 0.0 1.0) -1e+02))))
  (Audio|PlaySoundatLocation "/Game/Resouce/SE_MissileExplosion01.SE_MissileExplosion01" (Transformation|GetActorLocation) "0, 0, 0" 1.0 1.0 0.0 0 0 0))