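; Physics-sphere enemy that chases the player, wanders when out of range and self-destructs at close range.
; Tick steers velocity and facing, jumping when the player is higher.
; Reaching attack range starts an accelerating beep and eye-flash fuse, then a radial blast launches nearby physics actors, characters and fellow bugs.
; Fast impacts or blasts briefly stun it; hitting a Wall-tagged actor while stunned kills it and adds score.
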(event EventBeginPlay
  (bind _returnvalue (Rendering|Material|CreateDynamicMaterialInstance (Variables|Default|GetSphere1) 0 0 "None" :!class /Script/Engine.PrimitiveComponent))
  (Variables|Default|SetmyMaterial _returnvalue))

(event Collision|EventActorBeginOverlap
  (params (OtherActor :type Actor%20Object%20Reference)))

(event EventTick
  (params (DeltaSeconds :type Float%20%28single-precision%29))
  (CallFunction|AAAAA DeltaSeconds)
  (if (Variables|Default|GetisDamage)
    (Utilities|FlowControl|Delay 2.0)
    (Variables|Default|SetisDamage false)
    (else
      (CallFunction|MakeGoVector)
      (CallFunction|EnemyMove)
      (CallFunction|EnemyRotate)
      (CallFunction|EnemyJump))))

(event Collision|EventHit
  (params (MyComp :type Primitive%20Component%20Object%20Reference) (Other :type Actor%20Object%20Reference) (OtherComp :type Primitive%20Component%20Object%20Reference) (bSelfMoved :type Boolean) (HitLocation :type Vector :default "0, 0, 0") (HitNormal :type Vector :default "0, 0, 0") (NormalImpulse :type Vector :default "0, 0, 0") (Hit :type Hit%20Result%20Structure%20%28by%20ref%29))
  (CallFunction|OnHit Other))

(fn ConstructionScript)

(fn EnemyMove
  (bind _returnvalue (Transformation|GetVelocity))
  (bind _govector (Variables|Default|GetgoVector))
  (bind _returnvalue_2 (* _govector 1e+02))
  (bind _returnvalue_3 (+ _returnvalue _returnvalue_2))
  (Physics|SetPhysicsLinearVelocity (Variables|Default|GetSphere) (Math|Vector|MakeVector (Math|Float|Clamp(Float) (.x _returnvalue_3) (* (Variables|Default|GetcurrentSpeed) -1.0) (Variables|Default|GetcurrentSpeed)) (Math|Float|Clamp(Float) (.y _returnvalue_3) (* (Variables|Default|GetcurrentSpeed) -1.0) (Variables|Default|GetcurrentSpeed)) (.z _returnvalue_3)) false "None"))

(fn EnemyRotate
  (Transformation|SetActorRotation (Math|Rotator|MakeRotfromXZ (Variables|Default|GetgoVector) (Math|Vector|MakeVector 0.0 0.0 1.0))))

(fn EnemyJump
  (if (not (Variables|Default|GetisJump))
    (if (Variables|Default|GetisUp)
      (Physics|SetPhysicsLinearVelocity (Variables|Default|GetSphere) (+ (Transformation|GetVelocity) (Math|Vector|MakeVector 0.0 0.0 6e+02)) false "None")
      (Variables|Default|SetisJump true))))

(fn MakeGoVector
  (bind _returnvalue (Transformation|GetActorLocation))
  (bind _returnvalue_2 (Game|Player|GetPlayerPawn 0))
  (bind _returnvalue_3 (Transformation|GetActorLocation _returnvalue_2))
  (bind _returnvalue_4 (- _returnvalue_3 _returnvalue))
  (bind _returnvalue_5 (Math|Vector|MakeVector (.x _returnvalue_4) (.y _returnvalue_4) (.z _returnvalue_4)))
  (bind _returnvalue_6 (Math|Vector|VectorLength _returnvalue_5))
  (Variables|Default|SetgoVector (Math|Vector|Normalize (Math|Vector|MakeVector (.x _returnvalue_4) (.y _returnvalue_4) 0.0)))
  (bind _output_get (Variables|Default|SettargetDistance _returnvalue_6))
  (Variables|Default|SetisUp (> (.z _returnvalue_4) (Variables|Default|GetupHeight)))
  (Variables|Default|SetisChase (< _returnvalue_6 (Variables|Default|GetchaseRange)))
  (if (Variables|Default|GetisChase)
    (if (> _output_get (Variables|Default|GetattacRange))
      (Variables|Default|SetcurrentSpeed (Math|Float|Lerp (Variables|Default|GetcurrentSpeed) (Variables|Default|GetmaxSpeed) 0.1))
      (else
        (Variables|Default|SetcurrentSpeed (Math|Float|Lerp (Variables|Default|GetcurrentSpeed) 0.0 0.1))
        (Variables|Default|SetisBoom true)))
    (else
      (Variables|Default|SetcurrentSpeed (Math|Float|Lerp (Variables|Default|GetcurrentSpeed) (Variables|Default|GetmaxSpeed) 0.1))
      (bind _output_get_2 (Variables|Default|SetrandomVectorcurrentTime (+ (Utilities|Time|GetWorldDeltaSeconds) (Variables|Default|GetrandomVectorcurrentTime))))
      (if (> _output_get_2 (Variables|Default|GetrandomVectorChangeTime))
        (bind _output_get_3 (Variables|Default|SetrandomVector (Math|Vector|Normalize (Math|Vector|MakeVector (Math|Random|RandomFloatinRange -1.0 1.0) (Math|Random|RandomFloatinRange -1.0 1.0) 0.0))))
        (Variables|Default|SetgoVector _output_get_3)
        (Variables|Default|SetrandomVectorcurrentTime 0.0)
        (else
          (Variables|Default|SetgoVector (Variables|Default|GetrandomVector)))))))

(fn OnHit
  (params (other :type Actor%20Object%20Reference))
  (bind _returnvalue (Transformation|GetVelocity other))
  (if (Actor|ActorHasTag other "Wall")
    (if (Variables|Default|GetisDamage)
      (bind _asbp_time_game_character (Utilities|Casting|CastToBP_TimeGameCharacter (Game|Player|GetPlayerPawn 0)))
      (Default|AddScore _asbp_time_game_character)
      (Audio|PlaySound2D "/Game/Resouce/Sound/SE_EnemyDie.SE_EnemyDie" 1.0 1.0 0.0 0 0)
      (Niagara|SpawnSystematLocation "/Game/Resouce/Particle/NA_EnemyDie.NA_EnemyDie" (Transformation|GetActorLocation))
      (Actor|DestroyActor))
    (elif (> (Math|Vector|VectorLength _returnvalue) 6e+02)
      (Variables|Default|SetisDamage true)
      (Physics|SetPhysicsLinearVelocity (Variables|Default|GetSphere) (+ (Transformation|GetVelocity) _returnvalue) false "None")
      (elif (<= (.z (Transformation|GetVelocity)) 0.0)
        (Variables|Default|SetisJump false)))))

(fn AAAAA
  (params (deltaTime :type Float%20%28single-precision%29))
  (if (Variables|Default|GetisBoom)
    (Variables|Default|SetcurrentTime (+ deltaTime (Variables|Default|GetcurrentTime)))
    (if (> (Variables|Default|GetpitCount) 17)
      (CallFunction|Explosion)
      (elif (> (Variables|Default|GetcurrentTime) (Variables|Default|GetboomPitTime))
        (Audio|PlaySoundatLocation "/Game/Resouce/beep-08b.beep-08b" (Transformation|GetActorLocation) "0, 0, 0" 1.0 1.0 0.0 0 0 0)
        (Rendering|Material|SetVectorParameterValue (Variables|Default|GetmyMaterial) "EyeColor" (Class|KismetMathLibrary|HSVtoRGB 0.0 1.0 3e+01 1.0) :!class /Script/Engine.MaterialInstanceDynamic)
        (Variables|Default|SetcurrentTime 0.0)
        (Variables|Default|SetpitCount (+ (Variables|Default|GetpitCount) 1))
        (if (> (Variables|Default|GetpitCount) 7)
          (Variables|Default|SetboomPitTime 0.1)
          (elif (> (Variables|Default|GetpitCount) 2)
            (Variables|Default|SetboomPitTime 0.2)))
        (elif (> (Variables|Default|GetcurrentTime) (Variables|Default|GetpitTime))
          (Rendering|Material|SetVectorParameterValue (Variables|Default|GetmyMaterial) "EyeColor" (Class|KismetMathLibrary|HSVtoRGB 0.0 1.0 1.0 1.0) :!class /Script/Engine.MaterialInstanceDynamic))))))

(fn ColorReset)

(fn Explosion
  (bind _returnvalue (Transformation|GetActorLocation))
  (bind _outactors (Collision|SphereOverlapActors (Transformation|GetActorLocation) 7e+02 (Utilities|Array|MakeArray "ObjectTypeQuery4" "ObjectTypeQuery3") 0))
  (for _array_element _outactors
    (bind _asstatic_mesh_component (Utilities|Casting|CastToStaticMeshComponent (Variables|/Script/Engine.Actor|GetRootComponent _array_element))
      (:then
        (Physics|AddRadialImpulse _asstatic_mesh_component (Transformation|GetActorLocation) 7e+02 1e+03 "RIF_Constant" true)
        (bind _asbp_use_inverse_actor (Utilities|Casting|CastToBP_UseInverseActor _array_element))
        (Default|GetStopPhysics _asbp_use_inverse_actor (Math|Vector|Normalize (- (Transformation|GetActorLocation _asbp_use_inverse_actor) (Transformation|GetActorLocation))) (* 1000 (/ (- 7e+02 (Math|Vector|VectorLength (- (Transformation|GetActorLocation _asbp_use_inverse_actor) (Transformation|GetActorLocation)))) 7e+02))))
      (:CastFailed
        (bind _ascharacter (Utilities|Casting|CastToCharacter _array_element)
          (:then
            (Character|Jump _ascharacter)
            (Utilities|FlowControl|Sequence
              (:then_0
                (if (== (Game|GetPlayerCharacter 0) _ascharacter)
                  (Variables|Default|SetjumpPower 2e+03)
                  (else
                    (Variables|Default|SetjumpPower 1e+03))))
              (:then_1
                (Variables|/Script/Engine.MovementComponent|SetVelocity (Variables|/Script/Engine.Character|GetCharacterMovement _ascharacter) (+ (Pawn|Components|CharacterMovement|GetLastUpdateVelocity (Variables|/Script/Engine.Character|GetCharacterMovement _ascharacter)) (* (Math|Vector|Normalize (- (Transformation|GetActorLocation _ascharacter) (Transformation|GetActorLocation))) (* (/ (- 7e+02 (Math|Vector|VectorLength (- (Transformation|GetActorLocation _ascharacter) (Transformation|GetActorLocation)))) 7e+02) (Variables|Default|GetjumpPower))))))))
          (:CastFailed
            (bind _asbp_enemy_bug_bug_bug (Utilities|Casting|CastToBP_EnemyBugBugBug _array_element))
            (Variables|BP_EnemyBugBugBug_C|SetisDamage _asbp_enemy_bug_bug_bug true)
            (Physics|AddRadialImpulse (Variables|BP_EnemyBugBugBug_C|GetSphere _asbp_enemy_bug_bug_bug) (Transformation|GetActorLocation) 7e+02 1e+03 "RIF_Constant" true))))))
  (Niagara|SpawnSystematLocation "/Game/Resouce/Particle/NA_Gltich.NA_Gltich" _returnvalue)
  (Audio|PlaySoundatLocation "/Game/Resouce/Sound/SE_Explosion.SE_Explosion" _returnvalue "0, 0, 0" 1.0 1.0 0.0 0 0 0)
  (Actor|DestroyActor))