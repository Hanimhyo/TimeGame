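; BP_Spawn_EnemyBug is a timed spawner that keeps dropping BP_EnemyBugBugBug enemies into the level.
; Tick accumulates delta time into CurrentTime and, once it exceeds CreateTime, spawns a bug and resets the counter.
; Each bug appears high up at a random world-space X/Y within a fixed square around the origin, independent of the spawner's own location.
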(event EventBeginPlay)

(event Collision|EventActorBeginOverlap
  (params (OtherActor :type Actor%20Object%20Reference)))

(event EventTick
  (params (DeltaSeconds :type Float%20%28single-precision%29))
  (bind _output_get (Variables|Default|SetcurrentTime (+ DeltaSeconds (Variables|Default|GetcurrentTime))))
  (if (> _output_get (Variables|Default|GetcreateTime))
    (Game|SpawnActorfromClass "/Game/BluePrints/BP_EnemyBugBugBug.BP_EnemyBugBugBug_C" (Math|Transform|MakeTransform (Math|Vector|MakeVector (Math|Random|RandomFloatinRange -4e+03 4e+03) (Math|Random|RandomFloatinRange -4e+03 4e+03) 3e+03) "0, 0, 0" "1,1,1") "Undefined" 0 0)
    (Variables|Default|SetcurrentTime 0.0)))

(fn ConstructionScript)