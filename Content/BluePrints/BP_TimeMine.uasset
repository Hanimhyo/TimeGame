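; Timed mine actor that blinks red and beeps, faster in the last two seconds, then explodes.
; Tick runs the countdown and blink loop, compensating for global time dilation to keep real-time pace.
; The explosion radially impulses nearby static-mesh-root actors, passes distance-scaled push to BP_UseInverseActor via GetStopPhysics, spawns effects and destroys itself.
; EnemyBoom and PlayerBoom are empty stubs.
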(event Custom|ColorReset
  ;[1 1 1] Timer
  (Utilities|FlowControl|DoOnce false) ; enters at Reset
)

(event Custom|Explosion
  (bind _returnvalue (Transformation|GetActorLocation))
  ;[1 1 1] EXPLOSION!
  (bind _outactors (Collision|SphereOverlapActors (Transformation|GetActorLocation) 7e+02 (Utilities|Array|MakeArray "ObjectTypeQuery4" "ObjectTypeQuery3") 0))
  (for _array_element _outactors
    (bind _asstatic_mesh_component (Utilities|Casting|CastToStaticMeshComponent (Variables|/Script/Engine.Actor|GetRootComponent _array_element)))
    (Physics|AddRadialImpulse _asstatic_mesh_component (Transformation|GetActorLocation) 7e+02 1.5e+03 "RIF_Constant" true)
    (bind _asbp_use_inverse_actor (Utilities|Casting|CastToBP_UseInverseActor _array_element))
    (Default|GetStopPhysics _asbp_use_inverse_actor (Math|Vector|Normalize (- (Transformation|GetActorLocation _asbp_use_inverse_actor) (Transformation|GetActorLocation))) (* 1500 (/ (- 7e+02 (Math|Vector|VectorLength (- (Transformation|GetActorLocation _asbp_use_inverse_actor) (Transformation|GetActorLocation)))) 7e+02))))
  (Niagara|SpawnSystematLocation "/Game/Resouce/Particle/NA_Gltich.NA_Gltich" _returnvalue)
  (Audio|PlaySoundatLocation "/Game/Resouce/SE_MissileExplosion01.SE_MissileExplosion01" _returnvalue "0, 0, 0" 1.0 1.0 0.0 0 0 0)
  (Actor|DestroyActor))

(event EventBeginPlay
  ;[1 1 1] Start
  (bind _returnvalue (Rendering|Material|CreateDynamicMaterialInstance (Variables|Default|GetStaticMesh) 0 0 "None" :!class /Script/Engine.PrimitiveComponent))
  (Variables|Default|SetmyMaterial _returnvalue))

(event EventTick
  (params (DeltaSeconds :type Float%20%28single-precision%29))
  ;[1 1 1] Timer
  (bind _output_get (Variables|Default|SetcurrentTime (+ (* DeltaSeconds (/ 1.0 (Class|GameplayStatics|GetGlobalTimeDilation))) (Variables|Default|GetcurrentTime))))
  (if (> _output_get (Variables|Default|GetexposionTime))
    (CallFunction|Explosion)
    (else
      (Utilities|FlowControl|DoOnce false
        (:Completed
          (Utilities|FlowControl|Delay (* (Variables|Default|GetboomPitTime) (Class|GameplayStatics|GetGlobalTimeDilation)))
          (Rendering|Material|SetVectorParameterValue (Variables|Default|GetmyMaterial) "Color" (Math|Conversions|ToLinearColor(Color) (Variables|Default|Getred_Color)) :!class /Script/Engine.MaterialInstanceDynamic)
          (Audio|PlaySoundatLocation "/Game/Resouce/beep-08b.beep-08b" (Transformation|GetActorLocation) "0, 0, 0" 1.0 1.0 0.0 0 0 0)
          (Utilities|FlowControl|Delay (* (Variables|Default|GetpitTime) (Class|GameplayStatics|GetGlobalTimeDilation)))
          (Rendering|Material|SetVectorParameterValue (Variables|Default|GetmyMaterial) "Color" (Math|Conversions|ToLinearColor(Color) (Variables|Default|Getwhite_Color)) :!class /Script/Engine.MaterialInstanceDynamic)
          (if (> (+ (Variables|Default|GetcurrentTime) 2.0) (Variables|Default|GetexposionTime))
            (Variables|Default|SetboomPitTime (* 0.1 (Class|GameplayStatics|GetGlobalTimeDilation)))
            (if (> (+ (Variables|Default|GetcurrentTime) 1.0) (Variables|Default|GetexposionTime))
              (Variables|Default|SetboomPitTime (* 0.05 (Class|GameplayStatics|GetGlobalTimeDilation)))))
          (CallFunction|ColorReset))))))

(fn ConstructionScript)

(fn EnemyBoom
  (params (actor :type Actor%20Object%20Reference)))

(fn PlayerBoom)