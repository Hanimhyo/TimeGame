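; Physics actor that continuously records its recent motion and can rewind through it when OnInverseStart fires.
; Tick fills fixed-length rolling arrays of location, rotation and linear and angular velocity at a fixed 60-frame step.
; Rewinding disables physics, tints the mesh and lerps backwards through the recorded transforms.
; At the oldest sample it re-enables physics with the saved velocities, restores the color and rebuilds the history.
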(event Custom|OnInverseStart
  (Variables|Default|SetisInverse true)
  (Variables|Default|SetcurrentTime_delta 0.0)
  (CallFunction|PhyscisNoSetting)
  (bind _returnvalue (Rendering|Material|CreateDynamicMaterialInstance (Variables|Default|GetStaticMesh) 0 0 "None" :!class /Script/Engine.PrimitiveComponent))
  (Rendering|Material|SetVectorParameterValue _returnvalue "Color" "(R=0.802083,G=0.456364,B=0.376058,A=1.000000)" :!class /Script/Engine.MaterialInstanceDynamic))

(event EventBeginPlay
  (CallFunction|ArraySetting))

(event Collision|EventActorBeginOverlap
  (params (OtherActor :type Actor%20Object%20Reference)))

(event EventTick
  (params (DeltaSeconds :type Float%20%28single-precision%29))
  (if (Variables|Default|GetisInverse)
    (CallFunction|InverseMove DeltaSeconds)
    (else
      (CallFunction|NowandSaveArray DeltaSeconds))))

(fn ConstructionScript)

(fn NowandSaveArray
  (params (deltaTime :type Float%20%28single-precision%29))
  (bind _output_get (Variables|Default|SetcurrentTime_delta (+ (Variables|Default|GetcurrentTime_delta) deltaTime)))
  (if (>= _output_get (Variables|Default|Get60frameTime))
    (for _index (range 0 (Math|Float|Truncate (- (/ (Variables|Default|GetcurrentTime_delta) (Variables|Default|Get60frameTime)) 1.0)))
      (Utilities|FlowControl|Sequence
        (:then_0
          (bind _output_get_2 (Variables|Default|SetnowLocation (Transformation|GetActorLocation)))
          (Utilities|Array|Add (Variables|Default|GetarrayLocation) _output_get_2)
          (Utilities|Array|RemoveIndex (Variables|Default|GetarrayLocation)))
        (:then_1
          (bind _output_get_3 (Variables|Default|SetnowRotation (Transformation|GetActorRotation)))
          (Utilities|Array|Add (Variables|Default|GetarrayRotation) _output_get_3)
          (Utilities|Array|RemoveIndex (Variables|Default|GetarrayRotation)))
        (:then_2
          (bind _returnvalue (Physics|GetPhysicsLinearVelocity (Variables|Default|GetStaticMesh) "None"))
          (bind _output_get_4 (Variables|Default|SetnowPhysicsVector _returnvalue))
          (Utilities|Array|Add (Variables|Default|GetarrayPhysicsVector) _output_get_4)
          (Utilities|Array|RemoveIndex (Variables|Default|GetarrayPhysicsVector)))
        (:then_3
          (bind _output_get_5 (Variables|Default|SetnowPhysicsAngle_rad (Class|PrimitiveComponent|GetPhysicsAngularVelocityinRadians (Variables|Default|GetStaticMesh) "None")))
          (Utilities|Array|Add (Variables|Default|GetarrayPhysicsAngle_rad) _output_get_5)
          (Utilities|Array|RemoveIndex (Variables|Default|GetarrayPhysicsAngle_rad)))))
    (Variables|Default|SetcurrentTime_delta (Math|Float|%(Float) (Variables|Default|GetcurrentTime_delta) (Variables|Default|Get60frameTime)))))

(fn ArraySetting
  (Utilities|FlowControl|Sequence
    (:then_0
      (bind _output_get (Variables|Default|SetnowLocation (Transformation|GetActorLocation)))
      (for _index (range 1 (Variables|Default|GettotalFrameLenght))
        (Utilities|Array|Add (Variables|Default|GetarrayLocation) _output_get)))
    (:then_1
      (bind _output_get_2 (Variables|Default|SetnowRotation (Transformation|GetActorRotation)))
      (for _index_2 (range 1 (Variables|Default|GettotalFrameLenght))
        (Utilities|Array|Add (Variables|Default|GetarrayRotation) _output_get_2)))
    (:then_2
      (bind _returnvalue (Physics|GetPhysicsLinearVelocity (Variables|Default|GetStaticMesh) "None"))
      (bind _output_get_3 (Variables|Default|SetnowPhysicsVector _returnvalue))
      (for _index_3 (range 1 (Variables|Default|GettotalFrameLenght))
        (Utilities|Array|Add (Variables|Default|GetarrayPhysicsVector) _output_get_3)))
    (:then_3
      (bind _output_get_4 (Variables|Default|SetnowPhysicsAngle_rad (Class|PrimitiveComponent|GetPhysicsAngularVelocityinRadians (Variables|Default|GetStaticMesh) "None")))
      (for _index_4 (range 1 (Variables|Default|GettotalFrameLenght))
        (Utilities|Array|Add (Variables|Default|GetarrayPhysicsAngle_rad) _output_get_4)))
    (:then_4
      (Variables|Default|SetnowFrameNum (- (Variables|Default|GettotalFrameLenght) 1)))))

(fn InverseMove
  (params (deltaTime :type Float%20%28single-precision%29))
  (bind _60frametime (Variables|Default|Get60frameTime))
  (Utilities|FlowControl|Sequence
    (:then_0
      (bind _output_get (Variables|Default|SetcurrentTime_delta (+ (Variables|Default|GetcurrentTime_delta) deltaTime)))
      (if (>= _output_get (Variables|Default|Get60frameTime))
        (if (< (- (Variables|Default|GetnowFrameNum) (Math|Float|Truncate (/ (Variables|Default|GetcurrentTime_delta) _60frametime))) 0)
          (bind _output_get_2 (Variables|Default|SetnowFrameNum 0))
          (Variables|Default|SetnextFrameNum (- _output_get_2 1))
          (Variables|Default|SetcurrentTime_delta (Math|Float|%(Float) (Variables|Default|GetcurrentTime_delta) _60frametime))
          (else
            (bind _output_get_3 (Variables|Default|SetnowFrameNum (- (Variables|Default|GetnowFrameNum) (Math|Float|Truncate (/ (Variables|Default|GetcurrentTime_delta) _60frametime)))))
            (Variables|Default|SetnextFrameNum (- _output_get_3 1))
            (Variables|Default|SetcurrentTime_delta (Math|Float|%(Float) (Variables|Default|GetcurrentTime_delta) _60frametime))))))
    (:then_1
      (if (not (== (Variables|Default|GetnextFrameNum) -1))
        (Transformation|SetActorLocation (Math|Vector|Lerp(Vector) (Utilities|Array|Get(acopy) (Variables|Default|GetarrayLocation) (Variables|Default|GetnowFrameNum)) (Utilities|Array|Get(acopy) (Variables|Default|GetarrayLocation) (Variables|Default|GetnextFrameNum)) (Variables|Default|GetcurrentTime_delta)) false false)))
    (:then_2
      (if (not (== (Variables|Default|GetnextFrameNum) -1))
        (Transformation|SetActorRotation (Math|Rotator|Lerp(Rotator) (Utilities|Array|Get(acopy) (Variables|Default|GetarrayRotation) (Variables|Default|GetnowFrameNum)) (Utilities|Array|Get(acopy) (Variables|Default|GetarrayRotation) (Variables|Default|GetnextFrameNum)) (Variables|Default|GetcurrentTime_delta)))))
    (:then_3
      (if (== (Variables|Default|GetnextFrameNum) -1)
        (Variables|Default|SetisInverse false)
        (Physics|SetSimulatePhysics (Variables|Default|GetStaticMesh) true)
        (Collision|SetCollisionEnabled (Variables|Default|GetStaticMesh) "QueryAndPhysics")
        (Physics|SetPhysicsLinearVelocity (Variables|Default|GetStaticMesh) (Utilities|Array|Get(acopy) (Variables|Default|GetarrayPhysicsVector) (Variables|Default|GetnowFrameNum)) false "None")
        (Class|PrimitiveComponent|SetPhysicsAngularVelocityinRadians (Variables|Default|GetStaticMesh) (Utilities|Array|Get(acopy) (Variables|Default|GetarrayPhysicsAngle_rad) (Variables|Default|GetnowFrameNum)) false "None")
        (CallFunction|ResetValue)
        (CallFunction|ClearArray)
        (CallFunction|ArraySetting)
        (bind _returnvalue (Rendering|Material|CreateDynamicMaterialInstance (Variables|Default|GetStaticMesh) 0 0 "None" :!class /Script/Engine.PrimitiveComponent))
        (Rendering|Material|SetVectorParameterValue _returnvalue "Color" "(R=1.000000,G=0.977000,B=1.000000,A=1.000000)" :!class /Script/Engine.MaterialInstanceDynamic)))))

(fn ClearArray
  (Utilities|FlowControl|Sequence
    (:then_0
      (Utilities|Array|Clear (Variables|Default|GetarrayLocation)))
    (:then_1
      (Utilities|Array|Clear (Variables|Default|GetarrayRotation)))
    (:then_2
      (Utilities|Array|Clear (Variables|Default|GetarrayPhysicsVector)))
    (:then_3
      (Utilities|Array|Clear (Variables|Default|GetarrayPhysicsAngle_rad)))))

(fn PhyscisNoSetting
  (Physics|SetSimulatePhysics (Variables|Default|GetStaticMesh) false))

(fn ResetValue
  (bind _totalframelenght (Variables|Default|GettotalFrameLenght))
  (Variables|Default|SetcurrentTime_delta 0.0)
  (Variables|Default|SetnowFrameNum (- _totalframelenght 1))
  (Variables|Default|SetnextFrameNum (- _totalframelenght 2)))