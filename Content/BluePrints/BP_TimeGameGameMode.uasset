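; Game mode for the time game that adds the crosshair widget and runs a fixed, delay-timed sequence of world states: low gravity, stop and inverse, each followed by a clear.
; SearchArray caches tagged background cubes' dynamic materials and UseInverse actors, re-adding the actors per cube.
; Each state recolors the materials and, except clear, notifies those actors.
; BeginPlay also rescales player and bug-enemy gravity, while Tick counts down GameTime.
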(event Custom|WorldClear
  (for _array_element (Variables|Default|GetbackGroundMaterials)
    (Rendering|Material|SetVectorParameterValue _array_element "LineColor" (Math|Conversions|ToLinearColor(Color) (Variables|Default|GetnormalColor)) :!class /Script/Engine.MaterialInstanceDynamic)
    (Rendering|Material|SetScalarParameterValue _array_element "Speed" 5e+01 :!class /Script/Engine.MaterialInstanceDynamic)))

(event Custom|WorldInverse
  (for _array_element (Variables|Default|GetbackGroundMaterials)
    (Rendering|Material|SetVectorParameterValue _array_element "LineColor" (Class|KismetMathLibrary|HSVtoRGB 0.0 1.0 5e+01 1.0) :!class /Script/Engine.MaterialInstanceDynamic))
  (for _array_element_2 (Variables|Default|GetinverseCubeActors)
    (Default|WorldInverse _array_element_2)))

(event Custom|WorldStop
  (for _array_element (Variables|Default|GetbackGroundMaterials)
    (Rendering|Material|SetVectorParameterValue _array_element "LineColor" (Class|KismetMathLibrary|HSVtoRGB 6e+01 1.0 5e+01 1.0) :!class /Script/Engine.MaterialInstanceDynamic)
    (Rendering|Material|SetScalarParameterValue _array_element "Speed" 0.0 :!class /Script/Engine.MaterialInstanceDynamic))
  (for _array_element_2 (Variables|Default|GetinverseCubeActors)
    (Default|WorldStop _array_element_2)))

(event Custom|WorldNoGravity
  (for _array_element (Variables|Default|GetbackGroundMaterials)
    (Rendering|Material|SetVectorParameterValue _array_element "LineColor" (Class|KismetMathLibrary|HSVtoRGB 2.4e+02 1.0 5e+01 1.0) :!class /Script/Engine.MaterialInstanceDynamic))
  (for _array_element_2 (Variables|Default|GetinverseCubeActors)
    (Default|WorldNoGravity _array_element_2)))

(event EventBeginPlay
  (bind _returnvalue (UserInterface|CreateWidget "/Game/BluePrints/WBP_CrossWidget.WBP_CrossWidget_C" (Game|GetPlayerController 0)))
  (UserInterface|Viewport|AddtoViewport _returnvalue 0)
  (Variables|/Script/Engine.PlayerController|SetbShowMouseCursor (Game|GetPlayerController 0) false)
  (Input|SetInputModeGameOnly (Game|GetPlayerController 0))
  (CallFunction|SearchArray)
  (Utilities|FlowControl|Delay 1e+01)
  (CallFunction|WorldNoGravity)
  (bind _asbp_time_game_character (Utilities|Casting|CastToBP_TimeGameCharacter (Game|Player|GetPlayerPawn 0)))
  (Variables|/Script/Engine.CharacterMovementComponent|SetGravityScale (Variables|/Script/Engine.Character|GetCharacterMovement _asbp_time_game_character) 0.166667)
  (bind _outactors (Actor|GetAllActorsOfClass "/Game/BluePrints/BP_BugEnemy.BP_BugEnemy_C"))
  (for _array_element _outactors
    (Variables|/Game/BluePrints/BP_BugEnemy.BP_BugEnemy_C|SetgravityValue _array_element -163.333328))
  (Utilities|FlowControl|Delay 15.0)
  (CallFunction|WorldClear)
  (bind _asbp_time_game_character_2 (Utilities|Casting|CastToBP_TimeGameCharacter (Game|Player|GetPlayerPawn 0)))
  (Variables|/Script/Engine.CharacterMovementComponent|SetGravityScale (Variables|/Script/Engine.Character|GetCharacterMovement _asbp_time_game_character_2) 1.0)
  (bind _outactors_2 (Actor|GetAllActorsOfClass "/Game/BluePrints/BP_BugEnemy.BP_BugEnemy_C"))
  (for _array_element_2 _outactors_2
    (Variables|/Game/BluePrints/BP_BugEnemy.BP_BugEnemy_C|SetgravityValue _array_element_2 -9.8e+02))
  (Utilities|FlowControl|Delay 1e+01)
  (CallFunction|WorldStop)
  (Utilities|FlowControl|Delay 15.0)
  (CallFunction|WorldClear)
  (Utilities|FlowControl|Delay 1e+01)
  (CallFunction|WorldInverse)
  (Utilities|FlowControl|Delay 3e+01)
  (CallFunction|WorldClear))

(event EventTick
  (params (DeltaSeconds :type Float%20%28single-precision%29))
  (Variables|Default|SetgameTime (- (Variables|Default|GetgameTime) DeltaSeconds)))

(fn ConstructionScript)

(fn SearchArray
  (bind _outactors (Actor|GetAllActorswithTag "BackGroundCube"))
  (bind _output_get (Variables|Default|SetbackGroundCube _outactors))
  (for _array_element _output_get
    (bind _returnvalue (Rendering|Material|CreateDynamicMaterialInstance (Actor|GetComponentbyClass _array_element "/Script/Engine.StaticMeshComponent") 0 0 "None" :!class /Script/Engine.PrimitiveComponent))
    (Utilities|Array|Add (Variables|Default|GetbackGroundMaterials) _returnvalue)
    (bind _outactors_2 (Actor|GetAllActorswithTag "UseInverse"))
    (for _array_element_2 _outactors_2
      (bind _asbp_use_inverse_actor (Utilities|Casting|CastToBP_UseInverseActor _array_element_2))
      (Utilities|Array|Add (Variables|Default|GetinverseCubeActors) _asbp_use_inverse_actor))))